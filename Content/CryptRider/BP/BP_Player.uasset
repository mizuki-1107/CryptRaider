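; BP_Player is the player Blueprint for CryptRider, handling object grabbing and the end-of-heist result.
; Grab input press and release call Grab and Release on the Grabber component.
; The Goal event uses HasItem, which checks the PhysicsHandle's grabbed actor for a tag, to test whether the player is holding the treasure.
; It then shows a success or failure widget and fades the camera to light grey with audio.
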(event Custom|Goal
  ;[1 1 1] ゴールしたとき、ゴール画面を表示
  (if (CallFunction|HasItem "Treasure")
    ;;[1 1 1] お宝をもっているとき、盗みに成功
    (bind _returnvalue (UserInterface|CreateWidget "/Game/CryptRider/UI/UI_Goal.UI_Goal_C"))
    (UserInterface|Viewport|AddtoViewport _returnvalue 0)
    (CameraFades|StartCameraFade (Game|GetPlayerCameraManager 0) 0.0 1.0 1.0 "(R=0.802083,G=0.802083,B=0.802083,A=1.000000)" true true)
    (else
      ;;[1 1 1] お宝をもっていないとき、盗みに失敗
      (bind _returnvalue_2 (UserInterface|CreateWidget "/Game/CryptRider/UI/UI_Goal_Fail.UI_Goal_Fail_C"))
      (UserInterface|Viewport|AddtoViewport _returnvalue_2 0)
      (CameraFades|StartCameraFade (Game|GetPlayerCameraManager 0) 0.0 1.0 1.0 "(R=0.802083,G=0.802083,B=0.802083,A=1.000000)" true true))))

(event EventBeginPlay)

(event Collision|EventActorBeginOverlap
  (params (OtherActor :type Actor%20Object%20Reference)))

(event EventTick
  (params (DeltaSeconds :type Float%20%28single-precision%29)))

(event Input|ActionEvents|InputActionGrab
  (params (Key :type Key%20Structure))
  (:Pressed
    (Class|Grabber|Grab (Variables|Default|GetGrabber)))
  (:Released
    (Class|Grabber|Release (Variables|Default|GetGrabber))))

(fn ConstructionScript
  (|CallParentFunction))

(fn HasItem
  (params (Tag :type String))
  (bind _physicshandle (Variables|Default|GetPhysicsHandle))
  (bind _returnvalue (Class|PhysicsHandleComponent|GetGrabbedComponent _physicshandle))
  (Utilities|IsValid _returnvalue
    (:Is%20Valid
      (return (Actor|ActorHasTag (Components|GetOwner _returnvalue) (Utilities|String|StringToName Tag))))
    (:Is%20Not%20Valid
      (return false))))